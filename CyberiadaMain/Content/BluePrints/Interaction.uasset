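; Interaction is a clickable actor with a Cube component that highlights under the cursor and responds to clicks when a character is nearby.
; Begin and end overlap events with any Character set and clear the IsPlayerNear flag, which gates a click handler that only prints a "Click" message.
; Cursor-over events add and remove an Outline overlay material on the cube, independent of proximity.
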(event MouseInput|EventActorBeginCursorOver
  (Rendering|Material|SetOverlayMaterial (Variables|Default|GetCube) "/Game/Materials/Outline.Outline" :!class /Script/Engine.MeshComponent))

(event MouseInput|EventActorEndCursorOver
  (Rendering|Material|SetOverlayMaterial (Variables|Default|GetCube) 0 :!class /Script/Engine.MeshComponent))

(event MouseInput|EventActorOnClicked
  (params (ButtonPressed :type Key%20Structure :default "None"))
  (if (Variables|Default|GetisPlayerNear)
    (Development|PrintText "Click")))

(event Collision|EventActorBeginOverlap
  (params (OtherActor :type Actor%20Object%20Reference))
  (Utilities|Casting|CastToCharacter OtherActor)
  (Variables|Default|SetisPlayerNear true))

(event Collision|EventActorEndOverlap
  (params (OtherActor :type Actor%20Object%20Reference))
  (Utilities|Casting|CastToCharacter OtherActor)
  (Variables|Default|SetisPlayerNear false))

(fn ConstructionScript)